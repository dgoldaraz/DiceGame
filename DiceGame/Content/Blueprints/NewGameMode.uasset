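; Game mode for a turn-based dice game between the player and an AI, with a random first turn.
; On BeginPlay it shows the HUD and splits BP_DiceMesh actors by X position, giving positive-X dice to the pawn's PlayerManager and keeping the rest as AI dice.
; Tick polls PlayerManager; when it is not the player's turn and its dice have stopped, it waits briefly, rolls the AI dice and switches turns.
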(event `self.ReceiveBeginPlay`
  (bind _output_get (set `self.PlayerManager` (`KismetArrayLibrary.Array_Get` (`self.K2_GetComponentsByClass` (`GameplayStatics.GetPlayerPawn` 0) "/Script/DiceGame.PlayerManager"))))
  (`PlayerManager.SetActiveTurn` _output_get (`KismetMathLibrary.RandomBool`))
  (bind _returnvalue (`|CreateWidget` "/Game/Blueprints/HUD.HUD_C"))
  (bind _output_get_2 (set `self.HUD_Ref` _returnvalue))
  (`UserWidget.AddToViewport` _output_get_2 0)
  (bind _outactors (`GameplayStatics.GetAllActorsOfClass` "/Game/FirstPersonCPP/Blueprints/BP_DiceMesh.BP_DiceMesh_C"))
  (for _array_element _outactors
    (bind _returnvalue_x (`KismetMathLibrary.BreakVector` (`self.K2_GetActorLocation` _array_element)))
    (if (> _returnvalue_x 0.0)
      (bind _item (`KismetArrayLibrary.Array_Get` (`self.K2_GetComponentsByClass` _array_element "/Script/DiceGame.DiceComponent")))
      (`PlayerManager.AddDice` (`self.PlayerManager`) _item)
      (else
        (`KismetArrayLibrary.Array_Add` (`self.AIDices`) _item)))))

(event `self.ReceiveTick`
  (params (DeltaSeconds :type "Float (single-precision)"))
  (bind _item (`KismetArrayLibrary.Array_Get` (`self.K2_GetComponentsByClass` (`GameplayStatics.GetPlayerPawn` 0) "/Script/DiceGame.PlayerManager")))
  (bind _returnvalue (`PlayerManager.GetPlayerTurn` _item))
  (bind _returnvalue_2 (`PlayerManager.AreDicesStop` _item))
  (if (and _returnvalue_2 (not _returnvalue))
    (`KismetSystemLibrary.Delay` 1.0)
    (`self.RollAIDices`)
    (`self.SwitchTurns`)))

(fn `RollAIDices`
  (for _array_element (`self.AIDices`)
    (`DiceComponent.RollDice` _array_element (0.0 0.0 0.0))))

(fn `SwitchTurns`
  (returns (PlayerTurn :type Boolean))
  (bind _item (`KismetArrayLibrary.Array_Get` (`self.K2_GetComponentsByClass` (`GameplayStatics.GetPlayerPawn` 0) "/Script/DiceGame.PlayerManager")))
  (bind _returnvalue (`PlayerManager.GetPlayerTurn` _item))
  (bind _returnvalue_2 (not _returnvalue))
  (`PlayerManager.SetActiveTurn` _item _returnvalue_2)
  (return _returnvalue_2))

(fn `UserConstructionScript`)